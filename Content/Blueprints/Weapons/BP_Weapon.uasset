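; BP_Weapon is a weapon Blueprint whose Fire event traces and spawns an Ammo actor.
; Fire runs a debug-drawn line trace against WorldStatic objects, 1000 units along the Arrow component's forward vector.
; The spawn transform comes from multiplying the Arrow's location by the trace end, so it carries no aim rotation and ignores whether anything was hit.
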(event `Fire`
  (bind _arrow (`self.Arrow`))
  (bind _returnvalue (`SceneComponent.K2_GetComponentLocation` _arrow))
  (bind _outhit (`KismetSystemLibrary.LineTraceSingleForObjects` :`Start` _returnvalue :`End` (+ _returnvalue (* (`KismetMathLibrary.GetForwardVector` (`SceneComponent.K2_GetComponentRotation` _arrow)) 1000.0)) :`ObjectTypes` (`|MakeArray` "ObjectTypeQuery1" :!type "EObjectTypeQuery Enum") :`DrawDebugType` "ForOneFrame"))
  (`|SpawnActorFromClass` (`self.Ammo`) (`KismetMathLibrary.Conv_VectorToTransform` (* (`SceneComponent.K2_GetComponentLocation` (`self.Arrow`)) (`.TraceEnd` (`GameplayStatics.BreakHitResult` _outhit)))) "Undefined" "MultiplyWithRoot" null null))

(fn `UserConstructionScript`)